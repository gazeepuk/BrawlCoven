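; Gameplay Ability for warriors in a turn-based battle, which ends the owning warrior's turn when the ability ends.
; Activation is placeholder logic: the authority resolves the battle player controller from the warrior's player index and checks for a selected warrior, with only debug prints on either network side.
; On end, it finds the CombatComponent on the ability system component's owner and calls ServerEndWarriorTurn.
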(event `self.K2_ActivateAbility`
  (bind _asbc_warrior_base (cast `BC_WarriorBase` (`self.GetOwningActorFromActorInfo`)))
  (`self.K2_HasAuthority`
    (:`True`
      (bind _returnvalue (`GameplayStatics.GetPlayerController` (`BC_WarriorBase.GetPlayerIndex` _asbc_warrior_base)))
      (`/Engine/EditorBlueprintResources/StandardMacros.IsValid` _returnvalue
        (:`Is Valid`
          (bind _asbp_battle_player_controller (cast `/Game/Blueprints/PlayerControllers/BP_BattlePlayerController` _returnvalue))
          (`/Engine/EditorBlueprintResources/StandardMacros.IsValid` (`BC_BattlePlayerController.GetSelectedWarrior` _asbp_battle_player_controller)
            (:`Is Valid`
              (`KismetSystemLibrary.PrintString` "Slay"))))))
    (:`False`
      (`KismetSystemLibrary.PrintString` "SOS"))))

(event `self.K2_OnEndAbility`
  (params (bWasCancelled :type Boolean))
  (bind _asbc_warrior_base (cast `BC_WarriorBase` (`ActorComponent.GetOwner` (`self.GetAbilitySystemComponentFromActorInfo`))))
  (bind _returnvalue (`Actor.GetComponentByClass` _asbc_warrior_base "/Script/BrawlCoven.CombatComponent"))
  (`/Engine/EditorBlueprintResources/StandardMacros.IsValid` _returnvalue
    (:`Is Valid`
      (`CombatComponent.Server_EndWarriorTurn` _returnvalue))))