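; BP_WarriorTest is a warrior Blueprint, apparently for testing, that orients itself once when play begins.
; After the parent BeginPlay it zeroes its rotation, then yaws 90 degrees left or right, or not at all.
; The sign of the Y difference between player 0's forward vector and its own picks the turn, so player facing matters rather than position.
; Tick, overlap and construction script are empty.
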(event `self.ReceiveBeginPlay`
  (bind (_returnvalue_roll _returnvalue_pitch _returnvalue_yaw) (`KismetMathLibrary.BreakRotator` (`self.K2_GetActorRotation`)))
  (bind (_returnvalue_x _returnvalue_y) (`KismetMathLibrary.BreakVector` (- (`self.GetActorForwardVector` (`GameplayStatics.GetPlayerPawn` 0)) (`self.GetActorForwardVector`))))
  (`parent.ReceiveBeginPlay`)
  (`self.K2_SetActorRotation` (struct))
  (`self.K2_SetActorRotation` (`KismetMathLibrary.MakeRotator` _returnvalue_roll _returnvalue_pitch (+ (* (`KismetMathLibrary.SignOfFloat` _returnvalue_y) -90.0) _returnvalue_yaw))))

(fn `UserConstructionScript`)